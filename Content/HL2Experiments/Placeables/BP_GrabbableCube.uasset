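; BP_GrabbableCube is a placeable physics cube that responds to lock-on, grab and release events.
; Grabbing suspends physics and gravity, and releasing restores both, then hides the mesh after a delay without destroying it.
; Releasing a lock re-enables physics first and gravity afterward.
; A dynamic material instance from the construction script drives the highlight color, lit on lock-on and dimmed on lock release or reset.
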(event `/Game/HL2Experiments/AR/Grab/BPI_Grabbable.PostRelease`
  (bind _staticmeshcomponent (`self.StaticMeshComponent`))
  ;[1 1 1] IMPLEMENT: Post Release
  (`PrimitiveComponent.SetSimulatePhysics` _staticmeshcomponent true)
  (`PrimitiveComponent.SetEnableGravity` _staticmeshcomponent true)
  (`KismetSystemLibrary.Delay` 12.0)
  (`SceneComponent.SetVisibility` _staticmeshcomponent false false))

(event `/Game/HL2Experiments/AR/Grab/BPI_Grabbable.PreGrab`
  (bind _staticmeshcomponent (`self.StaticMeshComponent`))
  ;[1 1 1] IMPLEMENT: Pre Grab
  (`PrimitiveComponent.SetSimulatePhysics` _staticmeshcomponent false)
  (`PrimitiveComponent.SetEnableGravity` _staticmeshcomponent false))

(event `/Game/HL2Experiments/AR/Grabbity/BPI_Grabbity.PreLockRelease`
  (bind _staticmeshcomponent (`self.StaticMeshComponent`))
  ;[1 1 1] IMPLEMENT: Pre Lock Release
  (`PrimitiveComponent.SetSimulatePhysics` _staticmeshcomponent true)
  (`PrimitiveComponent.SetEnableGravity` _staticmeshcomponent false)
  (`self.Dim`))

(event `/Game/HL2Experiments/AR/Grabbity/BPI_Grabbity.PostLockRelease`
  ;[1 1 1] IMPLEMENT: Post Lock Release
  (`PrimitiveComponent.SetEnableGravity` (`self.StaticMeshComponent`) true)
  (`self.Dim`))

(event `/Game/HL2Experiments/AR/Grabbity/BPI_Grabbity.PostLockOn`
  ;[1 1 1] IMPLEMENT: Post Lock On
  (`self.Highlight`))

(event `/Game/HL2Experiments/AR/Grabbity/BPI_Grabbity.Reset`
  ;[1 1 1] IMPLEMENT: Reset
  (`self.Dim`))

(fn `Dim`
  (bind _mid (`self.MID`))
  (`/Engine/EditorBlueprintResources/StandardMacros.IsValid` _mid
    (:`Is Valid`
      (`MaterialInstanceDynamic.SetVectorParameterValue` _mid "HighlightColor" (struct :`A` 1.0)))))

(fn `Highlight`
  (bind _mid (`self.MID`))
  (`/Engine/EditorBlueprintResources/StandardMacros.IsValid` _mid
    (:`Is Valid`
      (`MaterialInstanceDynamic.SetVectorParameterValue` _mid "HighlightColor" (struct :`R` 0.177083 :`G` 0.170196 :`A` 1.0)))))

(fn `UserConstructionScript`
  (bind _material (`self.Material`))
  (`/Engine/EditorBlueprintResources/StandardMacros.IsValid` _material
    (:`Is Valid`
      (bind _returnvalue (`KismetMaterialLibrary.CreateDynamicMaterialInstance` _material))
      (bind _output_get (set `self.MID` _returnvalue))
      (`PrimitiveComponent.SetMaterial` (`self.StaticMeshComponent`) 0 _output_get)
      (`self.Dim`))))