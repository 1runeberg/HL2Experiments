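; BP_Gesture_Tracker is an AR hand actor that tracks which fingertips touch the palm of one tracked hand.
; Every tick it moves palm and five fingertip collision components to their hand joint transforms, preserving each component's scale.
; Palm overlaps with the actor's own spheres maintain the FingersInPalm list and an IsIndexInPalm flag.
; On BeginPlay, child components tagged "Vis" are shown or hidden according to IsVisualizing.
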(event `self.ReceiveBeginPlay`
  (for _array_element (`SceneComponent.GetChildrenComponents` (`self.DefaultSceneRoot`) true)
    (if (`ActorComponent.ComponentHasTag` _array_element "Vis")
      (`SceneComponent.SetVisibility` _array_element (`self.IsVisualizing`) false))))

(event `self.ReceiveTick`
  (params (DeltaSeconds :type "Float (single-precision)"))
  (`self.Update Fingertips`))

(event `self.Palm.OnComponentBeginOverlap`
  (params (OverlappedComponent :type "PrimitiveComponent Object Reference") (OtherActor :type "Actor Object Reference") (OtherComp :type "PrimitiveComponent Object Reference") (OtherBodyIndex :type Integer) (bFromSweep :type Boolean) (SweepResult :type "HitResult Structure (by ref)"))
  (if (== OtherActor self)
    (bind _assphere_collision (cast `SphereComponent` OtherComp))
    (`KismetArrayLibrary.Array_AddUnique` (`self.FingersInPalm`) _assphere_collision)
    (if (== _assphere_collision (`self.Index`))
      (set `self.IsIndexInPalm` true))))

(event `self.Palm.OnComponentEndOverlap`
  (params (OverlappedComponent :type "PrimitiveComponent Object Reference") (OtherActor :type "Actor Object Reference") (OtherComp :type "PrimitiveComponent Object Reference") (OtherBodyIndex :type Integer))
  (if (== OtherActor self)
    (bind _assphere_collision (cast `SphereComponent` OtherComp))
    (`KismetArrayLibrary.Array_RemoveItem` (`self.FingersInPalm`) _assphere_collision)
    (if (== _assphere_collision (`self.Index`))
      (set `self.IsIndexInPalm` false))))

(fn `SetFingertipTransform`
  (params (FingertipCollision :type "SphereComponent Object Reference") (NewTransform :type "Transform Structure") (ApplyScale :type Boolean))
  (if ApplyScale
    (`SceneComponent.K2_SetWorldTransform` FingertipCollision (`KismetMathLibrary.MakeTransform` NewTransform_Location NewTransform_Rotation NewTransform_Scale) false false)
    (else
      (`SceneComponent.K2_SetWorldTransform` FingertipCollision (`KismetMathLibrary.MakeTransform` NewTransform_Location NewTransform_Rotation (`SceneComponent.K2_GetComponentScale` FingertipCollision)) false false))))

(fn `Update Fingertips`
  (`|ExecutionSequence`
    (:`then_0`
      (bind _transform (`WindowsMixedRealityHandTrackingFunctionLibrary.GetHandJointTransform` (`self.Hand`) "Palm"))
      (`self.SetFingertipTransform` (`self.Palm`) _transform))
    (:`then_1`
      (bind _transform_2 (`WindowsMixedRealityHandTrackingFunctionLibrary.GetHandJointTransform` (`self.Hand`) "IndexTip"))
      (`self.SetFingertipTransform` (`self.Index`) _transform_2))
    (:`then_2`
      (bind _transform_3 (`WindowsMixedRealityHandTrackingFunctionLibrary.GetHandJointTransform` (`self.Hand`) "MiddleTip"))
      (`self.SetFingertipTransform` (`self.Middle`) _transform_3))
    (:`then_3`
      (bind _transform_4 (`WindowsMixedRealityHandTrackingFunctionLibrary.GetHandJointTransform` (`self.Hand`) "RingTip"))
      (`self.SetFingertipTransform` (`self.Ring`) _transform_4))
    (:`then_4`
      (bind _transform_5 (`WindowsMixedRealityHandTrackingFunctionLibrary.GetHandJointTransform` (`self.Hand`) "LittleTip"))
      (`self.SetFingertipTransform` (`self.Pinky`) _transform_5))
    (:`then_5`
      (bind _transform_6 (`WindowsMixedRealityHandTrackingFunctionLibrary.GetHandJointTransform` (`self.Hand`) "ThumbTip"))
      (`self.SetFingertipTransform` (`self.Thumb`) _transform_6))))

(fn `UserConstructionScript`)