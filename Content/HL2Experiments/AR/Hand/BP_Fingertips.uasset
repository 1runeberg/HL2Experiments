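; BP_Fingertips keeps collision components glued to one tracked AR hand.
; Every tick it reads joint transforms for each finger's tip and a lower joint (intermediate, or proximal for the thumb) and moves the matching component there, keeping its scale.
; When IsWithPalm is set, Palm and Wrist components are also placed with PalmScale applied, both using the Palm keypoint.
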(event `self.ReceiveTick`
  (params (DeltaSeconds :type "Float (single-precision)"))
  (`self.Update Fingertips`))

(fn `SetFingertipTransform`
  (params (FingertipCollision :type "SphereComponent Object Reference") (NewTransform :type "Transform Structure") (ApplyScale :type Boolean))
  (if ApplyScale
    (`SceneComponent.K2_SetWorldTransform` FingertipCollision (`KismetMathLibrary.MakeTransform` NewTransform_Location NewTransform_Rotation NewTransform_Scale) false false)
    (else
      (`SceneComponent.K2_SetWorldTransform` FingertipCollision (`KismetMathLibrary.MakeTransform` NewTransform_Location NewTransform_Rotation (`SceneComponent.K2_GetComponentScale` FingertipCollision)) false false))))

(fn `Update Fingertips`
  (`|ExecutionSequence`
    (:`then_0`
      ;[1 1 1] Palm & Wrist
      (if (`self.IsWithPalm`)
        (bind _transform (`WindowsMixedRealityHandTrackingFunctionLibrary.GetHandJointTransform` (`self.Hand`) "Palm"))
        (`self.SetFingertipTransform` (`self.Palm`) (`KismetMathLibrary.MakeTransform` (.location _transform) (.rotation _transform) (`self.PalmScale`)) true)
        (bind _transform_2 (`WindowsMixedRealityHandTrackingFunctionLibrary.GetHandJointTransform` (`self.Hand`) "Palm"))
        (`self.SetFingertipTransform` (`self.Wrist`) (`KismetMathLibrary.MakeTransform` (.location _transform_2) (.rotation _transform_2) (`self.PalmScale`)) true)))
    (:`then_1`
      ;[1 1 1] Index
      (bind _transform_3 (`WindowsMixedRealityHandTrackingFunctionLibrary.GetHandJointTransform` (`self.Hand`) "IndexTip"))
      (`self.SetFingertipTransform` (`self.Index`) _transform_3)
      (bind _transform_4 (`WindowsMixedRealityHandTrackingFunctionLibrary.GetHandJointTransform` (`self.Hand`) "IndexIntermediate"))
      (`self.SetFingertipTransform` (`self.IndexMid`) _transform_4))
    (:`then_2`
      ;[1 1 1] Middle
      (bind _transform_5 (`WindowsMixedRealityHandTrackingFunctionLibrary.GetHandJointTransform` (`self.Hand`) "MiddleTip"))
      (`self.SetFingertipTransform` (`self.Middle`) _transform_5)
      (bind _transform_6 (`WindowsMixedRealityHandTrackingFunctionLibrary.GetHandJointTransform` (`self.Hand`) "MiddleIntermediate"))
      (`self.SetFingertipTransform` (`self.MiddleMid`) _transform_6))
    (:`then_3`
      ;[1 1 1] Ring
      (bind _transform_7 (`WindowsMixedRealityHandTrackingFunctionLibrary.GetHandJointTransform` (`self.Hand`) "RingTip"))
      (`self.SetFingertipTransform` (`self.Ring`) _transform_7)
      (bind _transform_8 (`WindowsMixedRealityHandTrackingFunctionLibrary.GetHandJointTransform` (`self.Hand`) "RingIntermediate"))
      (`self.SetFingertipTransform` (`self.RingMid`) _transform_8))
    (:`then_4`
      ;[1 1 1] Pinky
      (bind _transform_9 (`WindowsMixedRealityHandTrackingFunctionLibrary.GetHandJointTransform` (`self.Hand`) "LittleTip"))
      (`self.SetFingertipTransform` (`self.Pinky`) _transform_9)
      (bind _transform_10 (`WindowsMixedRealityHandTrackingFunctionLibrary.GetHandJointTransform` (`self.Hand`) "LittleIntermediate"))
      (`self.SetFingertipTransform` (`self.PinkyMid`) _transform_10))
    (:`then_5`
      (bind _transform_11 (`WindowsMixedRealityHandTrackingFunctionLibrary.GetHandJointTransform` (`self.Hand`) "ThumbTip"))
      (`self.SetFingertipTransform` (`self.Thumb`) _transform_11)
      (bind _transform_12 (`WindowsMixedRealityHandTrackingFunctionLibrary.GetHandJointTransform` (`self.Hand`) "ThumbProximal"))
      (`self.SetFingertipTransform` (`self.ThumbMid`) _transform_12))))

(fn `UserConstructionScript`)